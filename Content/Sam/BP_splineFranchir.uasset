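; Spline actor that moves the player character over an obstacle by vaulting (franchir), mounting (monter) or climbing (grimper).
; On BeginPlay it aligns to the player, then traces along a probe spline to find the obstacle and its height.
; It reshapes the movement spline to fit and picks a height-scaled vault timeline or a climb timeline to drive the player's location.
; Mounting cuts the vault short after a delay; `lacher` stops it.
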(event `lacher`
  (bind _returnvalue (`GameplayStatics.GetPlayerCharacter` 0))
  (bind _splinemonter (`self.splineMonter`))
  (bind _asbp_third_person_character (cast `/Game/ThirdPerson/Blueprints/BP_ThirdPersonCharacter` _returnvalue))
  (set `/Game/ThirdPerson/Blueprints/BP_ThirdPersonCharacter.isFranching` false _asbp_third_person_character)
  (bind (_direction _franchirmonter) (`Timeline|Timeline` :!via `Stop` :!label _label)
    (:`Update`
      (if (`self.arretMonte`)
        (bind _asbp_third_person_character_2 (cast `/Game/ThirdPerson/Blueprints/BP_ThirdPersonCharacter` _returnvalue))
        (set `/Game/ThirdPerson/Blueprints/BP_ThirdPersonCharacter.isMonting` false _asbp_third_person_character_2)
        (goto _label :!via `Stop`)
        (else
          (`self.K2_SetActorLocation` _returnvalue (`SplineComponent.GetLocationAtDistanceAlongSpline` _splinemonter (* (`SplineComponent.GetSplineLength` _splinemonter) _franchirmonter) "World") false false))))))

(event `self.ReceiveBeginPlay`
  (bind _returnvalue (`GameplayStatics.GetPlayerCharacter` 0))
  (bind _returnvalue_2 (`GameplayStatics.GetPlayerCharacter` 0))
  (bind _splinemonter (`self.splineMonter`))
  (bind _splinemonter_2 (`self.splineMonter`))
  (bind _splinemonter_3 (`self.splineMonter`))
  (bind _splinemonter_4 (`self.splineMonter`))
  (bind _returnvalue_3 (`SplineComponent.GetLocationAtSplinePoint` (`self.splineRC`) 0 "World"))
  (bind _returnvalue_4 (`SplineComponent.GetLocationAtSplinePoint` (`self.splineRC`) 1 "World"))
  (bind _mesh (`Character.Mesh` _returnvalue))
  (bind (_returnvalue_x _returnvalue_y) (`KismetMathLibrary.BreakVector` (* (- _returnvalue_4 _returnvalue_3) (0.05 0.05 0.0))))
  (`|ExecutionSequence`
    (:`then_0`
      (`SceneComponent.K2_SetWorldLocation` _splinemonter_4 (+ (`SceneComponent.K2_GetComponentLocation` _mesh) (0.0 0.0 90.0)) false false)
      (`SceneComponent.K2_SetWorldRotation` _splinemonter_4 (`KismetMathLibrary.MakeRotator` 0.0 0.0 (+ (.yaw (`SceneComponent.K2_GetComponentRotation` _mesh)) 90.0)) false false)
      (bind (_outhit _returnvalue_5) (`KismetSystemLibrary.LineTraceSingle` _returnvalue_3 _returnvalue_4 "TraceTypeQuery1" false (`|MakeArray` _returnvalue :!type "Actor Object Reference")))
      (if _returnvalue_5
        (bind (_bblockinghit _binitialoverlap _time _distance _location _impactpoint) (`GameplayStatics.BreakHitResult` _outhit))
        (set `self.Mod_spX-` (- (.x _returnvalue_4) (.x _impactpoint)))
        (set `self.Mod_spY-` (- (.y _returnvalue_4) (.y _impactpoint)))
        (set `self.Mod_spGrimperX-` (* (/ (- (.x _returnvalue_4) (.x _returnvalue_3)) 200.0) 65.0))
        (set `self.Mod_spGrimperY-` (* (/ (- (.y _returnvalue_4) (.y _returnvalue_3)) 200.0) 65.0))
        (`SceneComponent.K2_SetWorldLocation` (`self.splineRC`) (`KismetMathLibrary.MakeVector` (+ (.x _impactpoint) _returnvalue_x) (+ (.y _impactpoint) _returnvalue_y) (+ (.z _impactpoint) 165.0)) false false)
        (bind (_outhit_2 _returnvalue_6) (`KismetSystemLibrary.LineTraceSingle` (`SplineComponent.GetLocationAtSplinePoint` (`self.splineRC`) 0 "World") (`SplineComponent.GetLocationAtSplinePoint` (`self.splineRC`) 2 "World") "TraceTypeQuery1"))
        (if _returnvalue_6
          (bind (_bblockinghit_2 _binitialoverlap_2 _time_2 _distance_2 _location_2 _impactpoint_2 _normal _impactnormal _physmat _hitactor _hitcomponent _hitbonename _bonename _hititem _elementindex _faceindex _tracestart) (`GameplayStatics.BreakHitResult` _outhit_2))
          (set `self.spGramperZ` (+ (.z _tracestart) 50.0))
          (set `self.Mod_spZ*` (/ (- 155.0 (`KismetMathLibrary.FClamp` (- (- (.z _tracestart) (.z _location_2)) 10.0) 0.0 155.0)) 155.0))
          (`SplineComponent.SetLocationAtSplinePoint` (`self.splineMonter`) 1 (`self.getPrim` (`SplineComponent.GetLocationAtSplinePoint` _splinemonter_2 1 "World") 95.0 25.0) "World" true)
          (`SplineComponent.SetLocationAtSplinePoint` _splinemonter_2 2 (`self.getPrim` (`SplineComponent.GetLocationAtSplinePoint` _splinemonter_2 2 "World") 215.0 85.0) "World" true)
          (`SplineComponent.SetLocationAtSplinePoint` _splinemonter_2 3 (`self.getPrim` (`SplineComponent.GetLocationAtSplinePoint` _splinemonter_2 3 "World") 205.0 55.0) "World" true)
          (if _binitialoverlap_2
            (set `self.isGrimping` true :!label _label_2)
            (bind _asbp_third_person_character (cast `/Game/ThirdPerson/Blueprints/BP_ThirdPersonCharacter` (`GameplayStatics.GetPlayerCharacter` 0)))
            (set `/Game/ThirdPerson/Blueprints/BP_ThirdPersonCharacter.isGrimping` true _asbp_third_person_character)
            (`SplineComponent.RemoveSplinePoint` (`self.splineMonter`) 3 true)
            (`SplineComponent.RemoveSplinePoint` (`self.splineMonter`) 1 true)
            (`SplineComponent.SetLocationAtSplinePoint` _splinemonter_3 1 (`self.getPrimGrimper` (`SplineComponent.GetLocationAtSplinePoint` _splinemonter_3 2 "World")) "World" true)
            (bind (_direction _newtrack_0) (`Timeline|Grimper`)
              (:`Update`
                (`self.K2_SetActorLocation` _returnvalue_2 (`SplineComponent.GetLocationAtDistanceAlongSpline` _splinemonter (* (`SplineComponent.GetSplineLength` _splinemonter) _newtrack_0) "World") false false))
              (:`Finished`
                (bind _asbp_third_person_character_2 (cast `/Game/ThirdPerson/Blueprints/BP_ThirdPersonCharacter` _returnvalue_2))
                (set `/Game/ThirdPerson/Blueprints/BP_ThirdPersonCharacter.isGrimping` false _asbp_third_person_character_2)))
            (elif (> _distance_2 10.0)
              (set `self.isGrimping` false)
              (`TimelineComponent.SetPlayRate` (`self.Timeline`) (/ 1.0 (+ (`self.Mod_spZ*`) 0.25)))
              (goto _label :!via `PlayFromStart`)
              (elif (not (== _distance_2 0.0))
                (goto _label_2)))))))
    (:`then_1`
      (`KismetSystemLibrary.Delay` (* (`self.Mod_spZ*`) 0.66))
      (bind _asbp_third_person_character_3 (cast `/Game/ThirdPerson/Blueprints/BP_ThirdPersonCharacter` (`GameplayStatics.GetPlayerCharacter` 0)))
      (if (`/Game/ThirdPerson/Blueprints/BP_ThirdPersonCharacter.isMonting` _asbp_third_person_character_3)
        (set `self.arretMonte` true)))))

(event `Monter_Franchir_Grimper`
  (params (NewParam :type "Rotator Structure") (NewParam2 :type "Vector Structure")))

(fn `UserConstructionScript`)